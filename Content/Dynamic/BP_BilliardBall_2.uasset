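; Billiard ball actor with hand-written physics that gets knocked around by projectiles.
; A looping 100 Hz timer integrates its movement vector and teleports the sphere without sweep, applying gravity unless the last overlap set Grounded through a "Ground" tag.
; Projectile hits apply a restitution-based two-mass collision impulse along the player-to-ball direction, assuming a fixed projectile speed.
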(event OnComponentBeginOverlap(Sphere)
  (params (OverlappedComponent :type Primitive%20Component%20Object%20Reference) (OtherActor :type Actor%20Object%20Reference) (OtherComp :type Primitive%20Component%20Object%20Reference) (OtherBodyIndex :type Integer) (bFromSweep :type Boolean) (SweepResult :type Hit%20Result%20Structure%20%28by%20ref%29))
  (Utilities|FlowControl|Sequence
    (:then_1
      (Variables|Default|SetGrounded (Actor|ActorHasTag OtherActor "Ground")))))

(event OnComponentHit(Sphere)
  (params (HitComponent :type Primitive%20Component%20Object%20Reference) (OtherActor :type Actor%20Object%20Reference) (OtherComp :type Primitive%20Component%20Object%20Reference) (NormalImpulse :type Vector :default "0, 0, 0") (Hit :type Hit%20Result%20Structure%20%28by%20ref%29))
  (bind _returnvalue (Game|GetPlayerCharacter 0))
  (bind _returnvalue_2 (Transformation|GetActorLocation))
  (bind _returnvalue_3 (Transformation|GetActorLocation _returnvalue))
  (bind _returnvalue_4 (Math|Vector|GetUnitDirection(Vector) _returnvalue_3 _returnvalue_2))
  (bind _returnvalue_5 (* _returnvalue_4 5e+02))
  (bind _returnvalue_6 (* _returnvalue_4 _returnvalue_5))
  (if (Actor|ActorHasTag OtherActor "Projectile")
    (Development|PrintString "Hello")
    (bind _output_get (Variables|Default|SetMovementVector (+ (Variables|Default|GetMovementVector) (* _returnvalue_4 (- (+ (* (/ (- (Variables|Default|GetMass) (* (Variables|Default|Gete) (Variables|Default|GetM2))) (+ (Variables|Default|GetMass) (Variables|Default|GetM2))) (+ (.x (* _returnvalue_4 (Variables|Default|GetMovementVector))) (.y (* _returnvalue_4 (Variables|Default|GetMovementVector))) (.z (* _returnvalue_4 (Variables|Default|GetMovementVector))))) (* (+ (.x _returnvalue_6) (.y _returnvalue_6) (.z _returnvalue_6)) (/ (* (+ (Variables|Default|Gete) 1.0) (Variables|Default|GetM2)) (+ (Variables|Default|GetMass) (Variables|Default|GetM2))))) (+ (.x (* _returnvalue_4 (Variables|Default|GetMovementVector))) (.y (* _returnvalue_4 (Variables|Default|GetMovementVector))) (.z (* _returnvalue_4 (Variables|Default|GetMovementVector)))))))))
    (Development|PrintString (Utilities|String|ToString(Vector) _output_get) true true "(R=0.000000,G=0.660000,B=1.000000,A=1.000000)" 1e+01)))

(event Custom|PhysicsLULE
  ;[1 1 1] Gravitationskraft (uppdaters 100ggr i sekunden)
  (if (Variables|Default|GetGrounded)
    (Variables|Default|SetCurrentLocation (Math|Vector|MakeVector (.x (+ (Variables|Default|GetCurrentLocation) (/ (Variables|Default|GetMovementVector) 1e+02))) (.y (+ (Variables|Default|GetCurrentLocation) (/ (Variables|Default|GetMovementVector) 1e+02))) (.z (Variables|Default|GetCurrentLocation))))
    (bind _output_get (Variables|Default|SetMovementVector (Math|Vector|MakeVector (.x (Variables|Default|GetMovementVector)) (.y (Variables|Default|GetMovementVector)) 0.0)))
    (else
      (bind _output_get_2 (Variables|Default|SetCurrentLocation (Math|Vector|MakeVector (.x (+ (Variables|Default|GetCurrentLocation) (/ (Variables|Default|GetMovementVector) 1e+02))) (.y (+ (Variables|Default|GetCurrentLocation) (/ (Variables|Default|GetMovementVector) 1e+02))) (+ (- (.z (Variables|Default|GetMovementVector)) 0.0982) (.z (+ (Variables|Default|GetCurrentLocation) (/ (Variables|Default|GetMovementVector) 1e+02)))))))
      (Variables|Default|SetMovementVector (Math|Vector|MakeVector (.x (Variables|Default|GetMovementVector)) (.y (Variables|Default|GetMovementVector)) (- (.z (Variables|Default|GetMovementVector)) 0.0982)))))
  (Transformation|SetWorldLocation (Variables|Default|GetSphere) _output_get_2 false false))

(event Custom|RotationLULE
  (bind _sphere (Variables|Default|GetSphere))
  (bind _relativerotation (Variables|/Script/Engine.SceneComponent|GetRelativeRotation _sphere))
  (bind _returnvalue (+ (.yaw _relativerotation) 5.0))
  (Variables|Default|SetRotation (Math|Vector|MakeVector (.roll _relativerotation) (.pitch _relativerotation) _returnvalue))
  (Transformation|SetWorldRotation (Variables|Default|GetSphere) (Math|Rotator|MakeRotator (.roll _relativerotation) (.pitch _relativerotation) _returnvalue) false false))

(event EventBeginPlay
  ;[1 1 1] Sätter default saker och startar timern
  (Variables|Default|SetCurrentLocation (Transformation|GetActorLocation))
  (Variables|Default|SetRotation (Math|Rotator|GetRotationXVector (Transformation|GetWorldRotation (Variables|Default|GetSphere))))
  (Utilities|Time|SetTimerbyFunctionName 0 "PhysicsLULE" 0.01 true))

(event EventTick
  (params (DeltaSeconds :type Float%20%28single-precision%29)))

(fn ConstructionScript)