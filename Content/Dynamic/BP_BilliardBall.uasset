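; BP_BilliardBall is a billiard ball actor with a simple hand-written fall in place of engine physics.
; BeginPlay caches the Sphere's world location, and each Tick steps it down by a fixed amount, unscaled by delta time, until Grounded is set.
; Sphere begin overlap sets Grounded from the other actor's "Ground" tag; end overlap does nothing, and debug strings print throughout.
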(event OnComponentBeginOverlap(Sphere)
  (params (OverlappedComponent :type Primitive%20Component%20Object%20Reference) (OtherActor :type Actor%20Object%20Reference) (OtherComp :type Primitive%20Component%20Object%20Reference) (OtherBodyIndex :type Integer) (bFromSweep :type Boolean) (SweepResult :type Hit%20Result%20Structure%20%28by%20ref%29))
  (Development|PrintString "Hello")
  (Variables|Default|SetGrounded (Actor|ActorHasTag OtherActor "Ground"))
  (Development|PrintString "REEEEEEE"))

(event OnComponentEndOverlap(Sphere)
  (params (OverlappedComponent :type Primitive%20Component%20Object%20Reference) (OtherActor :type Actor%20Object%20Reference) (OtherComp :type Primitive%20Component%20Object%20Reference) (OtherBodyIndex :type Integer)))

(event Custom|PhysicsLULE
  (if (Variables|Default|GetGrounded)
    (Development|PrintString "Actor is touching ground")
    (else
      (Variables|Default|SetCurrentLocation (Math|Vector|MakeVector (.x (Variables|Default|GetCurrentLocation)) (.y (Variables|Default|GetCurrentLocation)) (- (.z (Variables|Default|GetCurrentLocation)) 1.0)))
      (Transformation|SetWorldLocation (Variables|Default|GetSphere) (Math|Vector|MakeVector (.x (Variables|Default|GetCurrentLocation)) (.y (Variables|Default|GetCurrentLocation)) (- (.z (Variables|Default|GetCurrentLocation)) 1.0)) false false))))

(event EventBeginPlay
  (Variables|Default|SetCurrentLocation (Transformation|GetWorldLocation (Variables|Default|GetSphere))))

(event Collision|EventActorBeginOverlap
  (params (OtherActor :type Actor%20Object%20Reference)))

(event EventTick
  (params (DeltaSeconds :type Float%20%28single-precision%29))
  (CallFunction|PhysicsLULE))

(fn ConstructionScript)