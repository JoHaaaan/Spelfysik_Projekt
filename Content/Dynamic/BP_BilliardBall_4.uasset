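; Billiard ball actor that simulates its own physics instead of using engine physics, moving and rotating its Sphere from a looping 0.01-second timer.
; Each step applies sliding friction when grounded or gravity otherwise, with Ground-tagged overlaps setting the grounded state.
; Restitution-based impulse formulas handle overlaps with BP_BilliardBall_2 and Projectile hits, which push along the player-to-ball direction.
; Rolling friction and torque-based spin are unwired, and debug prints remain.
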(event OnComponentBeginOverlap(Sphere)
  (params (OverlappedComponent :type Primitive%20Component%20Object%20Reference) (OtherActor :type Actor%20Object%20Reference) (OtherComp :type Primitive%20Component%20Object%20Reference) (OtherBodyIndex :type Integer) (bFromSweep :type Boolean) (SweepResult :type Hit%20Result%20Structure%20%28by%20ref%29))
  (Utilities|FlowControl|Sequence
    (:then_0
      (if (Actor|ActorHasTag OtherActor "VeryCool")
        (if (not (Variables|Default|GetOverlap))
          (Variables|Default|SetOverlap true)
          (bind _asbp_billiard_ball_2 (Utilities|Casting|CastToBP_BilliardBall_2 OtherActor)
            (:then
              (bind _output_get (Variables|Default|SetTempVector (Variables|/Game/Dynamic/BP_BilliardBall_2.BP_BilliardBall_2_C|GetMovementVector _asbp_billiard_ball_2)))
              (bind _output_get_2 (Variables|/Game/Dynamic/BP_BilliardBall_2.BP_BilliardBall_2_C|SetMovementVector _asbp_billiard_ball_2 (+ (Variables|/Game/Dynamic/BP_BilliardBall_2.BP_BilliardBall_2_C|GetMovementVector _asbp_billiard_ball_2) (* (Math|Vector|GetUnitDirection(Vector) (Variables|Default|GetCurrentLocation) (Variables|/Game/Dynamic/BP_BilliardBall_2.BP_BilliardBall_2_C|GetCurrentLocation _asbp_billiard_ball_2)) (- (+ (* (+ (.x (* (Variables|Default|GetMovementVector) (Math|Vector|GetUnitDirection(Vector) (Variables|Default|GetCurrentLocation) (Variables|/Game/Dynamic/BP_BilliardBall_2.BP_BilliardBall_2_C|GetCurrentLocation _asbp_billiard_ball_2)))) (.y (* (Variables|Default|GetMovementVector) (Math|Vector|GetUnitDirection(Vector) (Variables|Default|GetCurrentLocation) (Variables|/Game/Dynamic/BP_BilliardBall_2.BP_BilliardBall_2_C|GetCurrentLocation _asbp_billiard_ball_2)))) (.z (* (Variables|Default|GetMovementVector) (Math|Vector|GetUnitDirection(Vector) (Variables|Default|GetCurrentLocation) (Variables|/Game/Dynamic/BP_BilliardBall_2.BP_BilliardBall_2_C|GetCurrentLocation _asbp_billiard_ball_2))))) (/ (* (+ (Variables|Default|Gete) 1.0) (Variables|Default|GetMass)) (+ (Variables|Default|GetMass) (Variables|/Game/Dynamic/BP_BilliardBall_2.BP_BilliardBall_2_C|GetMass _asbp_billiard_ball_2)))) (* (+ (.x (* (Math|Vector|GetUnitDirection(Vector) (Variables|Default|GetCurrentLocation) (Variables|/Game/Dynamic/BP_BilliardBall_2.BP_BilliardBall_2_C|GetCurrentLocation _asbp_billiard_ball_2)) _output_get)) (.y (* (Math|Vector|GetUnitDirection(Vector) (Variables|Default|GetCurrentLocation) (Variables|/Game/Dynamic/BP_BilliardBall_2.BP_BilliardBall_2_C|GetCurrentLocation _asbp_billiard_ball_2)) _output_get)) (.z (* (Math|Vector|GetUnitDirection(Vector) (Variables|Default|GetCurrentLocation) (Variables|/Game/Dynamic/BP_BilliardBall_2.BP_BilliardBall_2_C|GetCurrentLocation _asbp_billiard_ball_2)) _output_get))) (/ (- (Variables|/Game/Dynamic/BP_BilliardBall_2.BP_BilliardBall_2_C|GetMass _asbp_billiard_ball_2) (* (Variables|Default|Gete) (Variables|Default|GetMass))) (+ (Variables|Default|GetMass) (Variables|/Game/Dynamic/BP_BilliardBall_2.BP_BilliardBall_2_C|GetMass _asbp_billiard_ball_2))))) (+ (.x (* (Math|Vector|GetUnitDirection(Vector) (Variables|Default|GetCurrentLocation) (Variables|/Game/Dynamic/BP_BilliardBall_2.BP_BilliardBall_2_C|GetCurrentLocation _asbp_billiard_ball_2)) _output_get)) (.y (* (Math|Vector|GetUnitDirection(Vector) (Variables|Default|GetCurrentLocation) (Variables|/Game/Dynamic/BP_BilliardBall_2.BP_BilliardBall_2_C|GetCurrentLocation _asbp_billiard_ball_2)) _output_get)) (.z (* (Math|Vector|GetUnitDirection(Vector) (Variables|Default|GetCurrentLocation) (Variables|/Game/Dynamic/BP_BilliardBall_2.BP_BilliardBall_2_C|GetCurrentLocation _asbp_billiard_ball_2)) _output_get))))))))
              (Variables|Default|SetMovementVector (+ (Variables|Default|GetMovementVector) (* (Math|Vector|GetUnitDirection(Vector) (Variables|Default|GetCurrentLocation) (Variables|/Game/Dynamic/BP_BilliardBall_2.BP_BilliardBall_2_C|GetCurrentLocation _asbp_billiard_ball_2)) (- (+ (* (/ (- (Variables|Default|GetMass) (* (Variables|Default|Gete) (Variables|/Game/Dynamic/BP_BilliardBall_2.BP_BilliardBall_2_C|GetMass _asbp_billiard_ball_2))) (+ (Variables|Default|GetMass) (Variables|/Game/Dynamic/BP_BilliardBall_2.BP_BilliardBall_2_C|GetMass _asbp_billiard_ball_2))) (+ (.x (* (Variables|Default|GetMovementVector) (Math|Vector|GetUnitDirection(Vector) (Variables|Default|GetCurrentLocation) (Variables|/Game/Dynamic/BP_BilliardBall_2.BP_BilliardBall_2_C|GetCurrentLocation _asbp_billiard_ball_2)))) (.y (* (Variables|Default|GetMovementVector) (Math|Vector|GetUnitDirection(Vector) (Variables|Default|GetCurrentLocation) (Variables|/Game/Dynamic/BP_BilliardBall_2.BP_BilliardBall_2_C|GetCurrentLocation _asbp_billiard_ball_2)))) (.z (* (Variables|Default|GetMovementVector) (Math|Vector|GetUnitDirection(Vector) (Variables|Default|GetCurrentLocation) (Variables|/Game/Dynamic/BP_BilliardBall_2.BP_BilliardBall_2_C|GetCurrentLocation _asbp_billiard_ball_2)))))) (* (+ (.x (* (Math|Vector|GetUnitDirection(Vector) (Variables|Default|GetCurrentLocation) (Variables|/Game/Dynamic/BP_BilliardBall_2.BP_BilliardBall_2_C|GetCurrentLocation _asbp_billiard_ball_2)) _output_get)) (.y (* (Math|Vector|GetUnitDirection(Vector) (Variables|Default|GetCurrentLocation) (Variables|/Game/Dynamic/BP_BilliardBall_2.BP_BilliardBall_2_C|GetCurrentLocation _asbp_billiard_ball_2)) _output_get)) (.z (* (Math|Vector|GetUnitDirection(Vector) (Variables|Default|GetCurrentLocation) (Variables|/Game/Dynamic/BP_BilliardBall_2.BP_BilliardBall_2_C|GetCurrentLocation _asbp_billiard_ball_2)) _output_get))) (/ (* (+ (Variables|Default|Gete) 1.0) (Variables|/Game/Dynamic/BP_BilliardBall_2.BP_BilliardBall_2_C|GetMass _asbp_billiard_ball_2)) (+ (Variables|Default|GetMass) (Variables|/Game/Dynamic/BP_BilliardBall_2.BP_BilliardBall_2_C|GetMass _asbp_billiard_ball_2))))) (+ (.x (* (Variables|Default|GetMovementVector) (Math|Vector|GetUnitDirection(Vector) (Variables|Default|GetCurrentLocation) (Variables|/Game/Dynamic/BP_BilliardBall_2.BP_BilliardBall_2_C|GetCurrentLocation _asbp_billiard_ball_2)))) (.y (* (Variables|Default|GetMovementVector) (Math|Vector|GetUnitDirection(Vector) (Variables|Default|GetCurrentLocation) (Variables|/Game/Dynamic/BP_BilliardBall_2.BP_BilliardBall_2_C|GetCurrentLocation _asbp_billiard_ball_2)))) (.z (* (Variables|Default|GetMovementVector) (Math|Vector|GetUnitDirection(Vector) (Variables|Default|GetCurrentLocation) (Variables|/Game/Dynamic/BP_BilliardBall_2.BP_BilliardBall_2_C|GetCurrentLocation _asbp_billiard_ball_2)))))))))
              (Utilities|FlowControl|Delay 1.0)
              (Variables|Default|SetOverlap false)
              (Variables|Default|SetTempVector "0, 0, 0"))
            (:CastFailed
              (Development|PrintString "cast failed"))))))
    (:then_1
      (Variables|Default|SetGrounded (Actor|ActorHasTag OtherActor "Ground")))))

(event OnComponentEndOverlap(Sphere)
  (params (OverlappedComponent :type Primitive%20Component%20Object%20Reference) (OtherActor :type Actor%20Object%20Reference) (OtherComp :type Primitive%20Component%20Object%20Reference) (OtherBodyIndex :type Integer))
  ;[1 1 1] misc
)

(event OnComponentHit(Sphere)
  (params (HitComponent :type Primitive%20Component%20Object%20Reference) (OtherActor :type Actor%20Object%20Reference) (OtherComp :type Primitive%20Component%20Object%20Reference) (NormalImpulse :type Vector :default "0, 0, 0") (Hit :type Hit%20Result%20Structure%20%28by%20ref%29))
  (bind _returnvalue (Game|GetPlayerCharacter 0))
  (bind _currentlocation (Variables|Default|GetCurrentLocation))
  (bind _returnvalue_2 (Transformation|GetActorLocation _returnvalue))
  (bind _returnvalue_3 (Math|Vector|GetUnitDirection(Vector) _returnvalue_2 _currentlocation))
  (bind _returnvalue_4 (* _returnvalue_3 5e+02))
  (bind _returnvalue_5 (* _returnvalue_3 _returnvalue_4))
  (if (Actor|ActorHasTag OtherActor "Projectile")
    (Variables|Default|SetMovementVector (+ (Variables|Default|GetMovementVector) (* _returnvalue_3 (- (+ (* (/ (- (Variables|Default|GetMass) (* (Variables|Default|Gete) (Variables|Default|GetM2))) (+ (Variables|Default|GetMass) (Variables|Default|GetM2))) (+ (.x (* _returnvalue_3 (Variables|Default|GetMovementVector))) (.y (* _returnvalue_3 (Variables|Default|GetMovementVector))) (.z (* _returnvalue_3 (Variables|Default|GetMovementVector))))) (* (+ (.x _returnvalue_5) (.y _returnvalue_5) (.z _returnvalue_5)) (/ (* (+ (Variables|Default|Gete) 1.0) (Variables|Default|GetM2)) (+ (Variables|Default|GetMass) (Variables|Default|GetM2))))) (+ (.x (* _returnvalue_3 (Variables|Default|GetMovementVector))) (.y (* _returnvalue_3 (Variables|Default|GetMovementVector))) (.z (* _returnvalue_3 (Variables|Default|GetMovementVector))))))))))

(event Custom|PhysicsLULE
  ;[1 1 1] Update
  (if (Variables|Default|GetGrounded)
    (CallFunction|CalculateForces)
    (bind _output_get (Variables|Default|SetMovementVector (* (+ (Variables|Default|GetMovementVector) (* (Variables|Default|GetAcceleration) 0.01)) "1.000000,1.000000,0.000000")))
    (if (< (.x _output_get) 0.0)
      (Variables|Default|SetMovementVector "0, 0, 0")
      (else
        (bind _output_get_2 (Variables|Default|SetCurrentLocation (Math|Vector|MakeVector (.x (+ (Variables|Default|GetCurrentLocation) (* (+ (Variables|Default|GetMovementVector) (* (Variables|Default|GetAcceleration) 0.01)) 0.01))) (.y (+ (Variables|Default|GetCurrentLocation) (* (+ (Variables|Default|GetMovementVector) (* (Variables|Default|GetAcceleration) 0.01)) 0.01))) (.z (Variables|Default|GetCurrentLocation)))))))
    (else
      (Variables|Default|SetCurrentLocation (Math|Vector|MakeVector (.x (+ (Variables|Default|GetCurrentLocation) (* (+ (Variables|Default|GetMovementVector) (* (Variables|Default|GetAcceleration) 0.01)) 0.01))) (.y (+ (Variables|Default|GetCurrentLocation) (* (+ (Variables|Default|GetMovementVector) (* (Variables|Default|GetAcceleration) 0.01)) 0.01))) (+ (- (.z (Variables|Default|GetMovementVector)) 0.0982) (.z (+ (Variables|Default|GetCurrentLocation) (* (+ (Variables|Default|GetMovementVector) (* (Variables|Default|GetAcceleration) 0.01)) 0.01))))))
      (Variables|Default|SetMovementVector (Math|Vector|MakeVector (.x (Variables|Default|GetMovementVector)) (.y (Variables|Default|GetMovementVector)) (- (.z (Variables|Default|GetMovementVector)) 0.0982)))))
  (bind _output_get_3 (Variables|Default|SetRotation (+ (Variables|Default|GetRotation) (* (Variables|Default|GetAngularVelocity) -0.01))))
  (Development|PrintString "Hello")
  (Transformation|SetWorldRotation (Variables|Default|GetSphere) (Math|Rotator|MakeRotator (Math|Trig|RadiansToDegrees (.y _output_get_3)) (Math|Trig|RadiansToDegrees (.x _output_get_3)) (Math|Trig|RadiansToDegrees (.z _output_get_3))) false false)
  (Transformation|SetWorldLocation (Variables|Default|GetSphere) _output_get_2 false false))

(event Custom|FartX
  (Variables|Default|SetMovementVector "50.000000,0.000000,0.000000"))

(event Custom|CalculateForces
  ;[1 1 1] CalculateForces
  (if (< (Math|Vector|VectorLength (- (Math|Vector|CrossProduct (Variables|Default|GetAngularVelocity) (* (Variables|Default|GetRadius) "0.000000,0.000000,-1.000000")) (Variables|Default|GetMovementVector))) 0.1)
    (if (> (Math|Vector|VectorLength (- (Math|Vector|CrossProduct (Variables|Default|GetAngularVelocity) (* (Variables|Default|GetRadius) "0.000000,0.000000,-1.000000")) (Variables|Default|GetMovementVector))) -0.1)
      (Variables|Default|SetRollPhase true)
      (Development|PrintString "Rullfas" true true "(R=0.000000,G=0.660000,B=1.000000,A=1.000000)" 1e+01)
      (else
        (bind _output_get (Variables|Default|SetFrictionForce (* (* (Math|Vector|Normalize (+ (* (Math|Vector|CrossProduct (Variables|Default|GetAngularVelocity) "0.000000,0.000000,-1.000000") (Variables|Default|GetRadius)) (Variables|Default|GetMovementVector))) -1.0) (* (Variables|Default|GetMass) 9.82 (Variables|Default|GetFrictionCoefficient))) :!label _label))
        (Variables|Default|SetAcceleration (/ (Math|Vector|MakeVector (.x _output_get) (.y _output_get) (.z _output_get)) (Variables|Default|GetMass)))
        (Development|PrintString (Utilities|String|ToString(Vector) (stale _output_get_2)))
        (bind _output_get_2 (Variables|Default|SetAngularVelocity (Math|Vector|MakeVector (/ (.x (Variables|Default|GetMovementVector)) (* (Variables|Default|GetRadius) 1e+02)) 0.0 0.0)))))
    (else
      (goto _label))))

(event EventBeginPlay
  (bind _sphere (Variables|Default|GetSphere))
  (bind _relativerotation (Variables|/Script/Engine.SceneComponent|GetRelativeRotation _sphere))
  ;[1 1 1] Sätter default saker och startar timern
  (Variables|Default|SetCurrentLocation (Transformation|GetActorLocation))
  (Variables|Default|SetRotation (Math|Vector|MakeVector (Math|Trig|DegreesToRadians (.roll _relativerotation)) (Math|Trig|DegreesToRadians (.pitch _relativerotation)) (Math|Trig|DegreesToRadians (.yaw _relativerotation))))
  (Utilities|Time|SetTimerbyFunctionName 0 "PhysicsLULE" 0.01 true))

(event Collision|EventActorBeginOverlap
  (params (OtherActor :type Actor%20Object%20Reference))
  ;[1 1 1] misc
)

(event EventTick
  (params (DeltaSeconds :type Float%20%28single-precision%29))
  ;[1 1 1] misc
)

(fn ConstructionScript)